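; Drivable vehicle pawn that can ram other vehicles, with flip recovery and mouse free-look.
; A box collider turns on from 20 km/h, and vehicle overlaps scale the other car's velocity by this car's forward vector.
; Tick updates speed and gear strings and resets roll after two seconds tipped over.
; BeginPlay hides in-car text and adds TestWidget; the spring arm rotates only while left mouse is held.
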(event OnComponentBeginOverlap(Box2_0)
  (params (OverlappedComponent :type Primitive%20Component%20Object%20Reference) (OtherActor :type Actor%20Object%20Reference) (OtherComp :type Primitive%20Component%20Object%20Reference) (OtherBodyIndex :type Integer) (bFromSweep :type Boolean) (SweepResult :type Hit%20Result%20Structure%20%28by%20ref%29))
  (if (!= OtherActor self)
    (bind _asbp_vehiculo (Utilities|Casting|CastToBP_Vehiculo OtherActor))
    (bind _returnvalue (Physics|GetPhysicsLinearVelocity (Variables|/Script/Engine.MovementComponent|GetUpdatedPrimitive (Variables|/Script/PhysXVehicles.WheeledVehicle|GetVehicleMovement _asbp_vehiculo)) "None"))
    (Physics|SetPhysicsLinearVelocity (Variables|/Script/Engine.MovementComponent|GetUpdatedPrimitive (Variables|/Script/PhysXVehicles.WheeledVehicle|GetVehicleMovement _asbp_vehiculo)) (* (* _returnvalue 2.5) (Transformation|GetActorForwardVector)) false "None")))

(event EventBeginPlay
  ;[1 1 1] Initialisation
  ;;[1 1 1] Disable both HUDs
  (Rendering|SetVisibility (Variables|Display|GetInCarGear_0) false false)
  (Rendering|SetVisibility (Variables||Display|GetInCarSpeed_0) false false)
  (Variables|Default|SetDefaultPosition_0 "-20.000000, 0, 0")
  (bind _returnvalue (UserInterface|CreateWidget "/Game/Proyect/Blueprints/TestWidget.TestWidget_C"))
  (UserInterface|Viewport|AddtoViewport _returnvalue 0))

(event EventTick
  (params (DeltaSeconds :type Float%20%28single-precision%29))
  (bind _returnvalue (Transformation|GetActorRotation))
  (bind _box2_0 (Variables|Default|GetBox2_0))
  ;[1 1 1] Update
  (Utilities|FlowControl|Sequence
    (:then_0
      (CallFunction|UpdateHUDStrings)
      (Utilities|Casting|CastToCarPlayerState (Variables|Default|GetPlayerState))
      (if (>= (* (Class|WheeledVehicleMovementComponent|GetForwardSpeed (Variables|Default|GetVehicleMovement)) 0.036) 2e+01)
        (Collision|SetCollisionEnabled _box2_0 "QueryAndPhysics")
        (else
          (Collision|SetCollisionEnabled _box2_0 "NoCollision"))))
    (:then_1
      (if (<= (Math|Vector|DotProduct (Transformation|GetActorUpVector) "0, 0,1.000000") 0.5)
        (Variables|Default|SetStuck_0 true)
        (Utilities|FlowControl|Delay 2.0)
        (if (Variables|Default|GetStuck_0)
          (Transformation|SetActorRotation (Math|Rotator|MakeRotator 0.0 (.pitch _returnvalue) (.yaw _returnvalue)) true))
        (else
          (Variables|Default|SetStuck_0 false))))))

(event Input|AxisEvents|InputAxisLookUp
  (params (AxisValue :type Float%20%28single-precision%29))
  (bind _springarmcomponent (Variables|Default|GetSpringArmComponent))
  ;[1 1 1] Free Camera Look
  (if (Game|Player|IsInputKeyDown (Game|GetPlayerController 0) "LeftMouseButton")
    (Transformation|AddRelativeRotation _springarmcomponent (Math|Rotator|MakeRotator 0.0 AxisValue (stale Input|AxisEvents|InputAxisLookRight AxisValue)) false false)
    (else
      (Transformation|SetRelativeRotation _springarmcomponent (Variables|Default|GetDefaultPosition_0) false false))))

(event Input|AxisEvents|InputAxisLookRight
  (params (AxisValue :type Float%20%28single-precision%29))
  (bind _springarmcomponent (Variables|Default|GetSpringArmComponent))
  ;[1 1 1] Free Camera Look
  (if (Game|Player|IsInputKeyDown (Game|GetPlayerController 0) "LeftMouseButton")
    (Transformation|AddRelativeRotation _springarmcomponent (Math|Rotator|MakeRotator 0.0 (stale Input|AxisEvents|InputAxisLookUp AxisValue) AxisValue) false false)
    (else
      (Transformation|SetRelativeRotation _springarmcomponent (Variables|Default|GetDefaultPosition_0) false false))))

(fn ConstructionScript)

(fn SetupIncarHUD
  ;[1 1 1] Setup Gear Display
  (Rendering|Components|TextRender|SetText (Variables|Display|GetInCarGear_0) (Utilities|Text|ToText(String) (Variables|Display|GetGear%20Display%20String_0)))
  (Rendering|Components|TextRender|SetTextRenderColor (Variables|Display|GetInCarGear_0) (Math|Conversions|ToColor(LinearColor) (Math|Color|SelectColor (Variables|Display|GetGearDisplayReverseColor_0) (Variables|Display|GetGearDisplayColor_0) (Variables|Game|GetInReverseGear_0))))
  ;[1 1 1] Setup speed display
  (Rendering|Components|TextRender|SetText (Variables||Display|GetInCarSpeed_0) (Utilities|Text|ToText(String) (Variables|Display|GetSpeed%20Display%20String_0))))

(fn UpdateHUDStrings
  (bind _vehiclemovement (Variables|Default|GetVehicleMovement))
  ;[1 1 1] Setup String for Speed
  (Variables|Display|SetSpeed%20Display%20String_0 (Utilities|String|Append (Utilities|String|ToString(Integer) (Math|Float|Floor (Math|Float|Absolute(Float) (* (Class|WheeledVehicleMovementComponent|GetForwardSpeed _vehiclemovement) 0.036)))) " km/h"))
  ;[1 1 1] Setup string for Gear
  (LocalVariables|SetCurrentGear (Class|WheeledVehicleMovementComponent|GetCurrentGear _vehiclemovement))
  (if (Variables|Game|GetInReverseGear_0) ; If zero display N else display R
    (Variables|Display|SetGear%20Display%20String_0 "R")
    (elif (> (LocalVariables|GetCurrentGear) 0)
      (Variables|Display|SetGear%20Display%20String_0 (Utilities|String|ToString(Integer) (LocalVariables|GetCurrentGear)))
      (else
        (Variables|Display|SetGear%20Display%20String_0 "N")))))