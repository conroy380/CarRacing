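; Straight road tile Blueprint for a racing game with a track built at runtime, exposing its arrow transform as the attach point.
; When a vehicle enters its box trigger, it asks RacingGameModeBase to add road and destroys itself after a five-second delay.
; During that delay, Tick shifts the emissive color of a dynamic material on the instanced mesh.
; BeginPlay creates that material and moves the static mesh to a fixed world height.
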(event OnComponentBeginOverlap(BoxComponent)
  (params (OverlappedComponent :type Primitive%20Component%20Object%20Reference) (OtherActor :type Actor%20Object%20Reference) (OtherComp :type Primitive%20Component%20Object%20Reference) (OtherBodyIndex :type Integer) (bFromSweep :type Boolean) (SweepResult :type Hit%20Result%20Structure%20%28by%20ref%29))
  (Utilities|Casting|CastToVehicleClass OtherActor)
  (bind _asracing_game_mode_base (Utilities|Casting|CastToRacingGameModeBase (Game|GetGameMode)))
  (Class|RacingGameModeBase|AddRoad _asracing_game_mode_base)
  (Variables|Default|SetStartCount true)
  (Utilities|FlowControl|Delay 5.0)
  (Actor|DestroyActor))

(event EventTick
  (params (DeltaSeconds :type Float%20%28single-precision%29))
  (if (Variables|Default|GetStartCount)
    (bind _output_get (Variables|Default|SetMin (+ (Variables|Default|GetMin) (* DeltaSeconds 0.25))))
    (bind _output_get_2 (Variables|Default|SetMax (- (Variables|Default|GetMax) (* DeltaSeconds 0.25))))
    (Rendering|Material|SetVectorParameterValue (Variables|Default|GetRoadColor) "EmisiveParam" (Utilities|Struct|MakeLinearColor _output_get _output_get_2 0.067277 1.0) :!class /Script/Engine.MaterialInstanceDynamic)))

(event EventBeginPlay
  (bind _staticmesh (Variables|Default|GetStaticMesh))
  (bind _returnvalue (Transformation|GetWorldLocation _staticmesh))
  (bind _returnvalue_2 (Rendering|Material|CreateDynamicMaterialInstance (Variables|Default|GetInstancedStaticMeshComponent) 0 "/Game/Proyect/StaticMeshes/Enviroment/Materials/M_Roads_Master_Inst.M_Roads_Master_Inst" "None" :!class /Script/Engine.PrimitiveComponent))
  (Variables|Default|SetRoadColor _returnvalue_2)
  (Transformation|SetWorldLocation _staticmesh (Math|Vector|MakeVector (.x _returnvalue) (.y _returnvalue) -1.9e+03) false false))

(fn ConstructionScript)

(fn GetAttachTransform
  (return (Transformation|GetWorldTransform (Variables|Default|GetArrowComponent))))