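; Game instance for the car racing game that handles creating, joining and ending multiplayer sessions.
; CreateSession takes a connection count and LAN flag, then on success opens the Lobby level as a listen server and stores the count as MaxPlayers.
; JoinSession and EndSession wrap the join and destroy session nodes, with create and join results printed to screen.
; The PlayersConnected RepNotify is an empty stub.
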(event Custom|CreateSession
  (params (PublicConnections :type Integer) (bUseLAN :type Boolean))
  (|Session (Game|GetPlayerController 0) PublicConnections bUseLAN
    (:OnSuccess
      (Development|PrintString "Session created")
      (Game|OpenLevel(byName) "Lobby" true "listen")
      (Variables|Default|SetMaxPlayers PublicConnections))
    (:OnFailure
      (Development|PrintString "Couldn't create session"))))

(event Custom|JoinSession
  (params (SessionToJoin :type Blueprint%20Session%20Result%20Structure%20%28by%20ref%29))
  (|JoinSession (Game|GetPlayerController 0) SessionToJoin
    (:OnSuccess
      (Development|PrintString "Joined the session"))
    (:OnFailure
      (Development|PrintString "Couldn't join the session"))))

(event Custom|EndSession
  (|DestroySession (Game|GetPlayerController 0)))

(fn OnRepPlayersConnected)